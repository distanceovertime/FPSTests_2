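; Note actor that travels through the level and bursts when damaged.
; Tick shifts it by a fixed step along negative world X each frame, without delta-time scaling, until it is hit.
; AnyDamage sets IsHit to halt movement and plays a timeline that drives its scale.
; When the timeline finishes, it spawns an explosion effect at its transform and destroys itself.
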(event EventBeginPlay)

(event Collision|EventActorBeginOverlap
  (params (OtherActor :type Actor%20Object%20Reference)))

(event EventTick
  (params (DeltaSeconds :type Float%20%28single-precision%29))
  (if (not (Variables|Default|GetisHit))
    (Transformation|SetActorLocation (+ (Transformation|GetActorLocation) "-38.500000, 0, 0") false false)))

(event Game|Damage|EventAnyDamage
  (params (Damage :type Float%20%28single-precision%29) (DamageType :type Damage%20Type%20Object%20Reference) (InstigatedBy :type Controller%20Object%20Reference) (DamageCauser :type Actor%20Object%20Reference))
  (bind _returnvalue (Transformation|GetActorTransform))
  (bind (_location _rotation _scale) (Math|Transform|BreakTransform _returnvalue))
  (Development|PrintString "hit")
  (Variables|Default|SetisHit true)
  (bind _newtrack_0 (Timeline|burst_timeline Play)
    (:Update
      (Transformation|SetActorScale3D _newtrack_0))
    (:Finished
      (Game|SpawnActorfromClass "/Game/StarterContent/Blueprints/Blueprint_Effect_Explosion.Blueprint_Effect_Explosion_C" (Math|Transform|MakeTransform _location _rotation (* _scale 1.0)) "Undefined" 0 0)
      (Actor|DestroyActor))))

(fn ConstructionScript)